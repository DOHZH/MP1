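; Enemy actor that damages the player on contact and awards score when shot.
; On overlap it destroys itself, then either subtracts HP from BP_Player or, for a bullet, destroys that bullet too.
; A player hit that drops HP to zero or below shows the restart display.
; A bullet hit finds the player through GetActorOfClass to add score.
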(event `self.ReceiveActorBeginOverlap`
  (params (OtherActor :type "Actor Object Reference"))
  (bind _asbp_player (cast `/Game/InfiniteMatrix/Blueprints/BP_Player` OtherActor)
    (:`then`
      (`self.K2_DestroyActor`)
      (bind _hp (`/Game/InfiniteMatrix/Blueprints/BP_Player.UpdateHp` _asbp_player false 10.0))
      (if (<= _hp 0.0)
        (`/Game/InfiniteMatrix/Blueprints/BP_Player.DisplayRestart` _asbp_player)))
    (:`CastFailed`
      (bind _asbullet (cast `/Game/InfiniteMatrix/Blueprints/bullet` OtherActor))
      (`self.K2_DestroyActor`)
      (`self.K2_DestroyActor` _asbullet)
      (bind _returnvalue (`GameplayStatics.GetActorOfClass` "/Game/InfiniteMatrix/Blueprints/BP_Player.BP_Player_C"))
      (`/Game/InfiniteMatrix/Blueprints/BP_Player.UpdateScore` _returnvalue true 2))))

(fn `UserConstructionScript`)