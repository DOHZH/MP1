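; BP_Tunnel is a tunnel segment with a rotating holed wall that the player must pass.
; Crossing its trigger scores, destroys the segment and asks the spawner for another.
; Hitting the wall costs score and health, showing restart at zero HP; bullets hitting the tunnel are destroyed.
; Helper functions randomize the wall and attach chance-based hearts and enemies using circle-equation positions, offsetting enemies from hearts; attachments are cleared on player overlap.
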(event OnComponentBeginOverlap(WallMesh)
  (params (OverlappedComponent :type Primitive%20Component%20Object%20Reference) (OtherActor :type Actor%20Object%20Reference) (OtherComp :type Primitive%20Component%20Object%20Reference) (OtherBodyIndex :type Integer) (bFromSweep :type Boolean) (SweepResult :type Hit%20Result%20Structure%20%28by%20ref%29))
  (bind _asbp_player (Utilities|Casting|CastToBP_Player OtherActor))
  (CallFunction|RemoveAllExtra)
  (if (not (Variables|/Game/InfiniteMatrix/Blueprints/BP_Player.BP_Player_C|GetIsDead _asbp_player))
    (Default|UpdateScore _asbp_player false 1)
    (bind _hp (Default|UpdateHp _asbp_player false 2e+01))
    (if (<= _hp 0.0)
      (Default|DisplayRestart _asbp_player)
      (Variables|/Game/InfiniteMatrix/Blueprints/BP_Player.BP_Player_C|SetIsDead _asbp_player true))))

(event OnComponentBeginOverlap(TriggerZone)
  (params (OverlappedComponent :type Primitive%20Component%20Object%20Reference) (OtherActor :type Actor%20Object%20Reference) (OtherComp :type Primitive%20Component%20Object%20Reference) (OtherBodyIndex :type Integer) (bFromSweep :type Boolean) (SweepResult :type Hit%20Result%20Structure%20%28by%20ref%29))
  (bind _asbp_player (Utilities|Casting|CastToBP_Player OtherActor))
  (CallFunction|RemoveAllExtra)
  (Default|SpawnTunnelatSpawnPoint (Variables|Default|GetTunnerlSpawner))
  (Actor|DestroyActor)
  (Default|UpdateScore _asbp_player true 1))

(event EventBeginPlay)

(event Collision|EventActorBeginOverlap
  (params (OtherActor :type Actor%20Object%20Reference))
  (bind _asbullet (Utilities|Casting|CastTobullet OtherActor))
  (Actor|DestroyActor _asbullet))

(event EventTick
  (params (DeltaSeconds :type Float%20%28single-precision%29))
  (Transformation|AddLocalRotation (Variables|组件|GetWallMesh) (Math|Rotator|MakeRotator (* DeltaSeconds (Variables|Default|GetRotateSpeed)) 0.0 0.0) false false))

(fn ConstructionScript)

(fn RandomizeWall
  (Components|StaticMesh|SetStaticMesh (Variables|组件|GetWallMesh) (Utilities|Select :Index (Math|Random|RandomIntegerinRange 0 3) :Option%200 "/Game/InfiniteMatrix/Meshes/SM_Hole_01.SM_Hole_01" :Option%201 "/Game/InfiniteMatrix/Meshes/SM_Hole_02.SM_Hole_02" :Option%202 "/Game/InfiniteMatrix/Meshes/SM_Hole_03.SM_Hole_03" :Option%203 "/Game/InfiniteMatrix/Meshes/SM_Hole_04.SM_Hole_04"))
  (Transformation|AddLocalRotation (Variables|组件|GetWallMesh) (Math|Rotator|MakeRotator (Math|Random|RandomFloatinRange 0.0 3.6e+02) 0.0 0.0) false false))

(fn RandomizeHeart
  (if (Math|Random|RandomBoolwithWeight 0.3)
    (bind _position (CallFunction|RandomPosition))
    (bind _returnvalue (Game|SpawnActorfromClass "/Game/InfiniteMatrix/Blueprints/Heart.Heart_C" (Math|Transform|MakeTransform _position "0,90.000000, 0" "0.050000,0.100000,0.050000") "Undefined" 0 0))
    (Transformation|AttachActorToActor _returnvalue self "None" "KeepRelative" "KeepRelative" "KeepRelative" true)
    (return _position)))

(fn RemoveAllExtra
  (for _array_element (Actor|GetAttachedActors self true)
    (Actor|DestroyActor _array_element)))

(fn RandomPosition
  (bind _returnvalue (Math|Random|RandomIntegerinRange -10 10))
  (bind _returnvalue_2 (* _returnvalue 20))
  (bind _returnvalue_3 (Math|Integer|Absolute(Integer) _returnvalue_2))
  (bind _returnvalue_4 (* _returnvalue_3 _returnvalue_3))
  (bind _returnvalue_5 (- 40000 _returnvalue_4))
  (bind _returnvalue_6 (Math|Conversions|ToFloat(Integer) _returnvalue_5))
  (bind _returnvalue_7 (|(sqrt(x)) _returnvalue_6))
  (return (Math|Vector|MakeVector (Math|Conversions|ToFloat(Integer) (* (Math|Random|RandomIntegerinRange 2 10) 200)) (Math|Conversions|ToFloat(Integer) _returnvalue_2) (Math|Float|SelectFloat _returnvalue_7 (- 0.0 _returnvalue_7) (Math|Random|RandomBool)))))

(fn RandomEnemy
  (params (heartposition :type Vector))
  (bind _returnvalue (Math|Vector|Equal(Vector) heartposition "0, 0, 0" 0.0001))
  (bind (_x _y _z) (Math|Vector|BreakVector heartposition))
  (if (Math|Random|RandomBoolwithWeight 0.5)
    (if _returnvalue
      (bind _position (CallFunction|RandomPosition)))
    (bind _returnvalue_2 (Game|SpawnActorfromClass "/Game/InfiniteMatrix/Blueprints/Enemy.Enemy_C" (Math|Transform|MakeTransform (Math|Vector|SelectVector _position (Math|Vector|MakeVector (Math|Float|SelectFloat (+ _x 5e+02) (- _x 2e+02) (< _x 1.2e+03)) (Math|Float|SelectFloat (+ _y 1e+02) (- _y 1e+02) (< _y 0.0)) (Math|Float|SelectFloat (+ _z 1e+02) (- _z 1e+02) (< _z 0.0))) _returnvalue) "0,-45.000000,-20.000000" "4.000000,4.000000,4.000000") "Undefined" 0 0))
    (Transformation|AttachActorToActor _returnvalue_2 self "None" "KeepRelative" "KeepRelative" "KeepRelative" true)))